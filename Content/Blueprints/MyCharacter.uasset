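; Player character Blueprint that handles walking, strafing, jumping, frame-time-scaled mouse look and a simple wall climb.
; While IsClimbing is set, the walk axis event line-traces a short distance ahead for WorldStatic objects.
; A hit with forward input triggers Jump and adds clamped upward velocity, while a miss sets gravity scale to normal.
; IsClimbing is only read in these graphs, never set.
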(event Input|ActionEvents|InputActionJump
  (:Pressed
    (Character|Jump)))

(fn ConstructionScript)

(event Input|AxisEvents|InputAxisAxisWalk
  (params (AxisValue :type Float%20%28single-precision%29))
  (bind _returnvalue (Transformation|GetActorLocation))
  (bind _charactermovement (Variables|Character|GetCharacterMovement))
  ;[1 1 1] Movement
  (Pawn|Input|AddMovementInput (Transformation|GetActorForwardVector) AxisValue)
  (if (Variables|Default|GetisClimbing)
    (bind _returnvalue_2 (Collision|LineTraceForObjects _returnvalue (+ _returnvalue (* (Transformation|GetActorForwardVector) 1e+02)) (Utilities|Array|MakeArray "ObjectTypeQuery1") false 0 "None"))
    (if _returnvalue_2
      (if (> (Input|AxisValues|GetAxisWalk) 0.1)
        (Character|Jump)
        (Variables|/Script/Engine.MovementComponent|SetVelocity _charactermovement (Math|Vector|ClampVectorSize (+ (Variables|/Script/Engine.MovementComponent|GetVelocity _charactermovement) "0, 0,100.000000") 0.0 5e+02)))
      (else
        (Variables|/Script/Engine.CharacterMovementComponent|SetGravityScale (Variables|Character|GetCharacterMovement) 1.0)))))

(event Input|AxisEvents|InputAxisAxisStrafe
  (params (AxisValue :type Float%20%28single-precision%29))
  ;[1 1 1] Movement
  (Pawn|Input|AddMovementInput (Transformation|GetActorRightVector) AxisValue))

(event Input|AxisEvents|InputAxisAxisMouseX
  (params (AxisValue :type Float%20%28single-precision%29))
  ;[1 1 1] Look
  (Pawn|Input|AddControllerYawInput (* AxisValue (Utilities|Time|GetWorldDeltaSeconds) (Variables|Default|GetBaseLookX))))

(event Input|AxisEvents|InputAxisAxisMouseY
  (params (AxisValue :type Float%20%28single-precision%29))
  ;[1 1 1] Look
  (Pawn|Input|AddControllerPitchInput (* (Utilities|Time|GetWorldDeltaSeconds) AxisValue (Variables|Default|GetBaseLookY))))