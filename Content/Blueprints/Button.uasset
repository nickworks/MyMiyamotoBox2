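; A Button actor that the player presses with the Use action while nearby and looking at its mesh.
; Overlapping Sphere1 enables input, caches the MyCharacter FPS camera and fades the active highlight on, while leaving disables input and fades it off.
; On Use, a short camera trace that hits the mesh calls ButtonPressed and starts a fade to purple.
; Timelines drive both fades through scalar parameters on a dynamic material created in the construction script.
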(event OnComponentBeginOverlap(Sphere1)
  (params (OtherActor :type Actor%20Object%20Reference) (OtherComp :type Primitive%20Component%20Object%20Reference) (OtherBodyIndex :type Integer) (bFromSweep :type Boolean) (SweepResult :type Hit%20Result%20Structure%20%28by%20ref%29))
  ;[1 1 1] Toggle Input
  (Input|EnableInput (Game|GetPlayerController 0))
  (bind _asmycharacter_c (Utilities|Casting|CastToMyCharacter OtherActor))
  (Variables|Default|SetPlayerCamera (Variables|/Game/Blueprints/MyCharacter.MyCharacter_C|GetCameraFPS _asmycharacter_c))
  (CallFunction|Fadeon))

(event OnComponentEndOverlap(Sphere1)
  (params (OtherActor :type Actor%20Object%20Reference) (OtherComp :type Primitive%20Component%20Object%20Reference) (OtherBodyIndex :type Integer))
  ;[1 1 1] Toggle Input
  (Input|DisableInput (Game|GetPlayerController 0))
  (CallFunction|FadeOff))

(event Custom|FadeToPurple
  ;[1 1 1] Fade To Purple
  (bind _blend (Timeline|TL-FadeToPurple PlayFromStart)
    (:Update
      (Rendering|Material|SetScalarParameterValue (Variables|Default|GetTheMaterial) "BlendUse" _blend :!class /Script/Engine.MaterialInstanceDynamic))))

(event Custom|FadeOff
  ;[1 1 1] FadeOff
  (bind _blend (Timeline|TL-FadeOff PlayFromStart)
    (:Update
      (Rendering|Material|SetScalarParameterValue (Variables|Default|GetTheMaterial) "BlendActive" _blend :!class /Script/Engine.MaterialInstanceDynamic))))

(event Custom|FadeOn
  ;[1 1 1] FadeOn
  (bind _blend (Timeline|TL-FadeOn PlayFromStart)
    (:Update
      (Rendering|Material|SetScalarParameterValue (Variables|Default|GetTheMaterial) "BlendActive" _blend :!class /Script/Engine.MaterialInstanceDynamic))))

(event Input|ActionEvents|InputActionUse
  (bind _playercamera (Variables|Default|GetPlayerCamera))
  (bind _returnvalue (Transformation|GetWorldLocation _playercamera))
  ;[1 1 1] Line Trace
  (:Pressed
    (bind (_outhit _returnvalue_2) (Collision|LineTraceByChannel _returnvalue (+ _returnvalue (* (Math|Vector|GetForwardVector _playercamera) 256.0)) "TraceTypeQuery1" false 0 "None" false))
    (if _returnvalue_2
      (if (== (Variables|Default|GetMesh) (.HitComponent (Collision|BreakHitResult _outhit)))
        (Default|CallButtonPressed)
        (CallFunction|FadetoPurple)))))

(fn ConstructionScript
  (bind _returnvalue (Rendering|Material|CreateDynamicMaterialInstance (Variables|Default|GetMesh) 0 0 :!class /Script/Engine.PrimitiveComponent))
  (Variables|Default|SetTheMaterial _returnvalue))